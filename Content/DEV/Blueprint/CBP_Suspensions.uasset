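; Suspension component for BP_Vehicle that simulates a wheel spring by applying force to the vehicle's HitBox at the component's location.
; Each tick it sphere-traces downward, ignoring BP_ObstacleHandler actors, and turns compression into an upward stiffness force plus damping from the frame-to-frame change.
; A DoOnce, reset after a short delay while airborne, plays a crash sound on ground contact.
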(event `self.ReceiveBeginPlay`
  (bind _asbp_vehicle (cast `/Game/DEV/Blueprint/BP_Vehicle` (`self.GetOwner`)))
  (set `self.RefBPVehicle` _asbp_vehicle)
  (set `self.RefHitBox` (`/Game/DEV/Blueprint/BP_Vehicle.HitBox` _asbp_vehicle))
  (`KismetSystemLibrary.DelayUntilNextTick`))

(event `self.ReceiveTick`
  (params (DeltaSeconds :type "Float (single-precision)"))
  (`self.SuspensionTrace`)
  (if (not (`self.bIsHittingGround`))
    (`KismetSystemLibrary.Delay` 0.25)
    (goto _label :!via `Reset`)))

(event `CrashSound`
  (params (Hit :type Boolean))
  (if Hit
    (`/Engine/EditorBlueprintResources/StandardMacros.DoOnce` false :!label _label
      (:`Completed`
        (`GameplayStatics.PlaySound2D` "/Game/Sound/SC_Crash.SC_Crash" 1.0 1.0 0.0 null null)))))

(fn `SuspensionTrace`
  (bind _returnvalue (`self.K2_GetComponentLocation`))
  (bind _suspensiondata (`self.SuspensionData`))
  (bind _suspensiondata_2 (`self.SuspensionData`))
  (bind _outactors (`GameplayStatics.GetAllActorsOfClass` "/Game/Developers/ahmet/Obstacles/BP_ObstacleHandler.BP_ObstacleHandler_C"))
  (set `self.Out Actors` _outactors)
  (bind (_outhit _returnvalue_2) (`KismetSystemLibrary.SphereTraceSingleForObjects` _returnvalue (- _returnvalue (* (`self.GetUpVector`) (`/Game/DEV/Blueprint/DataAsset/BP_DA_SuspensionSettings.SuspensionHeight` _suspensiondata))) (`/Game/DEV/Blueprint/DataAsset/BP_DA_SuspensionSettings.WheelRadius` _suspensiondata) (`/Game/DEV/Blueprint/DataAsset/BP_DA_SuspensionSettings.WalkableTypes` _suspensiondata) false (`self.Out Actors`) "ForOneFrame"))
  (set `self.bIsHittingGround` _returnvalue_2)
  (set `self.ForceLocation` _returnvalue)
  (bind (_bblockinghit _binitialoverlap _time _distance _location _impactpoint) (`GameplayStatics.BreakHitResult` _outhit))
  (`self.CrashSound` _bblockinghit)
  (set `self.Ratio` (`KismetMathLibrary.FClamp` (`KismetMathLibrary.SelectFloat` (- 1.0 (/ (`KismetMathLibrary.VSize` (- _impactpoint (`self.ForceLocation`))) (`/Game/DEV/Blueprint/DataAsset/BP_DA_SuspensionSettings.SuspensionHeight` (`self.SuspensionData`)))) 0.0 (`self.bIsHittingGround`))))
  (`PrimitiveComponent.AddForceAtLocation` (`self.RefHitBox`) (* (`self.GetUpVector`) (* (`/Game/DEV/Blueprint/DataAsset/BP_DA_SuspensionSettings.SuspensionForce` _suspensiondata_2) (+ (* (`self.Ratio`) (`/Game/DEV/Blueprint/DataAsset/BP_DA_SuspensionSettings.SuspensionStiffness` _suspensiondata_2)) (* (`/Game/DEV/Blueprint/DataAsset/BP_DA_SuspensionSettings.SuspensionDamping` _suspensiondata_2) (/ (- (`self.Ratio`) (`self.LastFrameRatio`)) (`GameplayStatics.GetWorldDeltaSeconds`)))))) (`self.ForceLocation`) "None")
  (set `self.LastFrameRatio` (`self.Ratio`)))