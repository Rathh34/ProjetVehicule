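; Scene component that simulates raycast-style suspension for BP_Vehicle at the component's own location.
; Each tick it sphere-traces along its down axis using SuspensionData's height, wheel radius and object types, with debug drawing.
; The hit distance becomes a clamped compression ratio, zero when airborne.
; A spring-damper force from that ratio and its rate of change pushes the vehicle's HitBox along the component's up axis.
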(event `self.ReceiveBeginPlay`
  (bind _asbp_vehicle (cast `/Game/DEV/Input/Blueprint/BP_Vehicle` (`self.GetOwner`)))
  (set `self.RefBPVehicle` _asbp_vehicle)
  (set `self.RefHitBox` (`/Game/DEV/Input/Blueprint/BP_Vehicle.HitBox` _asbp_vehicle)))

(event `self.ReceiveTick`
  (params (DeltaSeconds :type "Float (single-precision)"))
  (`self.SuspensionTrace`))

(fn `SuspensionTrace`
  (bind _returnvalue (`self.K2_GetComponentLocation`))
  (bind _suspensiondata (`self.SuspensionData`))
  (bind _suspensiondata_2 (`self.SuspensionData`))
  (bind (_outhit _returnvalue_2) (`KismetSystemLibrary.SphereTraceSingleForObjects` :`Start` _returnvalue :`End` (- _returnvalue (* (`self.GetUpVector`) (`/Game/DEV/Input/Blueprint/DataAsset/BP_DA_SuspensionSettings.SuspensionHeight` _suspensiondata))) :`Radius` (`/Game/DEV/Input/Blueprint/DataAsset/BP_DA_SuspensionSettings.WheelRadius` _suspensiondata) :`ObjectTypes` (`/Game/DEV/Input/Blueprint/DataAsset/BP_DA_SuspensionSettings.WalkableTypes` _suspensiondata) :`DrawDebugType` "ForOneFrame"))
  (set `self.bIsHittingGround` _returnvalue_2)
  (set `self.ForceLocation` _returnvalue)
  (set `self.Ratio` (`KismetMathLibrary.FClamp` (`KismetMathLibrary.SelectFloat` (- 1.0 (/ (`KismetMathLibrary.VSize` (- (`.ImpactPoint` (`GameplayStatics.BreakHitResult` _outhit)) (`self.ForceLocation`))) (`/Game/DEV/Input/Blueprint/DataAsset/BP_DA_SuspensionSettings.SuspensionHeight` (`self.SuspensionData`)))) 0.0 (`self.bIsHittingGround`))))
  (`PrimitiveComponent.AddForceAtLocation` (`self.RefHitBox`) (* (`self.GetUpVector`) (* (`/Game/DEV/Input/Blueprint/DataAsset/BP_DA_SuspensionSettings.SuspensionForce` _suspensiondata_2) (+ (* (`self.Ratio`) (`/Game/DEV/Input/Blueprint/DataAsset/BP_DA_SuspensionSettings.SuspensionStiffness` _suspensiondata_2)) (* (`/Game/DEV/Input/Blueprint/DataAsset/BP_DA_SuspensionSettings.SuspensionDamping` _suspensiondata_2) (/ (- (`self.Ratio`) (`self.LastFrameRatio`)) (`GameplayStatics.GetWorldDeltaSeconds`)))))) (`self.ForceLocation`) "None")
  (set `self.LastFrameRatio` (`self.Ratio`)))